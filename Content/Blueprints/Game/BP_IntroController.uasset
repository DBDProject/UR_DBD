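; BP_IntroController is the intro controller that preloads the L_Showcase1 map and connects to the game server before travelling there.
; On BeginPlay, the local controller binds D1NetGameMode's async load events and starts loading after a short delay.
; When loading ends, the GameInstance's NetManager tries a hardcoded IP, then falls back to a local server.
; The level opens either way, printing a debug-mode notice if both connections fail.
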(event `self.ReceiveBeginPlay`
  ; 초기 바인딩 작업 및 비동기 맵 로딩
  (if (`self.IsLocalController`)
    (bind _asd1net_game_mode (cast `D1NetGameMode` (`GameplayStatics.GetGameMode`)))
    (add `D1NetGameMode.OnAsyncLoadMapStart` _asd1net_game_mode (`|CreateDelegate` :!event `OnMapLoadStart`))
    (add `D1NetGameMode.OnAsyncLoadMapEnd` _asd1net_game_mode (`|CreateDelegate` :!event `OnMapLoadEnd`))
    (`KismetSystemLibrary.Delay` 1.0)
    (`D1NetGameMode.LoadAsyncGameMap` _asd1net_game_mode "L_Showcase1")))

(event `OnNetworkConnectionComplete`
  (params (bSuccess :type Boolean))
  ; 서버 접속 체크 이후 레벨 이동
  (if bSuccess
    (`KismetSystemLibrary.PrintString` "서버 접속 성공" true true (struct :`G` 0.66 :`B` 1.0 :`A` 1.0) 5.0)
    (else
      (`KismetSystemLibrary.PrintString` "서버가 존재하지 않으므로 디버그 모드로 접속합니다" true true (struct :`G` 0.66 :`B` 1.0 :`A` 1.0) 5.0)))
  (`KismetSystemLibrary.Delay` 1.0)
  (`GameplayStatics.OpenLevel` "L_Showcase1"))

(event `OnMapLoadStart`
  (`KismetSystemLibrary.PrintString` "로비맵 비동기 로딩 시작"))

(event `OnMapLoadEnd`
  (`KismetSystemLibrary.PrintString` "로비맵 비동기 로딩 완료 서버 접속")
  ; 서버 접속 비연결시 랜서버 접속
  (bind _asd1game_instance (cast `D1GameInstance` (`GameplayStatics.GetGameInstance`)))
  (bind _returnvalue (`D1GameInstance.GetNetManager` _asd1game_instance))
  (bind _returnvalue_2 (`DBDNetManager.Connect` _returnvalue "192.168.0.92" 5000 1500))
  (if _returnvalue_2
    (`self.OnNetworkConnectionComplete` true)
    (else
      (bind _returnvalue_3 (`DBDNetManager.ConnectLocalServer` _returnvalue 5000))
      (`self.OnNetworkConnectionComplete` _returnvalue_3))))

(fn `UserConstructionScript`)