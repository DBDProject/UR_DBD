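; Lobby player controller that creates the full-screen lobby UI and handles chat and killer/survivor matchmaking feedback.
; On BeginPlay it binds packet processor match and chat events plus game mode async map-load events, hiding debug buttons when connected.
; Server responses post system chat, and Enter focuses the chat box.
; Match ready stores server info in the game instance and async-loads L_Showcase; load completion only prints, as level-opening logic is unwired.
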(event `self.ReceiveBeginPlay`
  (bind _lobbygui (`self.LobbyGUI`))
  ; UI 등록
  (if (`self.IsLocalController`)
    (bind _returnvalue (`|CreateWidget` "/DBDUI/Blueprints/Lobby/WBP_LobbyFullScreenWidget.WBP_LobbyFullScreenWidget_C"))
    (`UserWidget.AddToViewport` _returnvalue 0)
    (set `self.LobbyGUI` _returnvalue)
    (set `self.bShowMouseCursor` true)
    ; Receive, 비동기 맵 로딩 이벤트 등록
    (bind _asd1game_instance (cast `D1GameInstance` (`GameplayStatics.GetGameInstance`)))
    (bind _returnvalue_2 (`D1GameInstance.GetNetManager` _asd1game_instance))
    (bind _returnvalue_3 (`DBDNetManager.GetPacketProcessor` _returnvalue_2))
    (add `DBDPacketProcessor.OnChatMessageReceived` _returnvalue_3 (`|CreateDelegate` :!event `OnChatRecved`))
    (add `DBDPacketProcessor.OnKillerMatchACK` _returnvalue_3 (`|CreateDelegate` :!event `OnKillerMatchACK`))
    (add `DBDPacketProcessor.OnSurvivorMatchACK` _returnvalue_3 (`|CreateDelegate` :!event `OnSurvivorMatchACK`))
    (add `DBDPacketProcessor.OnMatchAbandoned` _returnvalue_3 (`|CreateDelegate` :!event `OnMatchAbandoned`))
    (add `DBDPacketProcessor.OnMatchCancelACK` _returnvalue_3 (`|CreateDelegate` :!event `OnMatchCancelACK`))
    (add `DBDPacketProcessor.OnMatchReady` _returnvalue_3 (`|CreateDelegate` :!event `OnMatchReady`))
    (bind _asd1net_game_mode (cast `D1NetGameMode` (`GameplayStatics.GetGameMode`)))
    (add `D1NetGameMode.OnAsyncLoadMapStart` _asd1net_game_mode (`|CreateDelegate` :!event `OnAsyncLoadStart`))
    (add `D1NetGameMode.OnAsyncLoadMapEnd` _asd1net_game_mode (`|CreateDelegate` :!event `OnAsyncLoadEnd`))
    ; 네트워크 연결 시 디버그 UI 비활성화
    (bind _asd1game_instance_2 (cast `D1GameInstance` (`GameplayStatics.GetGameInstance`)))
    (bind _returnvalue_4 (`D1GameInstance.GetNetManager` _asd1game_instance_2))
    (if (`DBDNetManager.IsConnected` _returnvalue_4)
      (`|ExecutionSequence`
        (:`then_0`
          (`Widget.SetVisibility` (`/DBDUI/Blueprints/Lobby/WBP_LobbyFullScreenWidget.WBP_Button` _lobbygui) "Hidden"))
        (:`then_1`
          (`Widget.SetVisibility` (`/DBDUI/Blueprints/Lobby/WBP_LobbyFullScreenWidget.WBP_Button_2` _lobbygui) "Hidden"))
        (:`then_2`
          (`Widget.SetVisibility` (`/DBDUI/Blueprints/Lobby/WBP_LobbyFullScreenWidget.WBP_Button_3` _lobbygui) "Hidden"))
        (:`then_3`
          (`Widget.SetVisibility` (`/DBDUI/Blueprints/Lobby/WBP_LobbyFullScreenWidget.WBP_Button_4` _lobbygui) "Hidden"))
        (:`then_4`
          (`Widget.SetVisibility` (`/DBDUI/Blueprints/Lobby/WBP_LobbyFullScreenWidget.WBP_Button_1` _lobbygui) "Hidden"))))))

(event `OnChatRecved`
  (params (message :type String))
  ; 채팅 받을 때 이벤트
  (`/DBDUI/Blueprints/BP_TestChat.Send Chat` (`/DBDUI/Blueprints/Lobby/WBP_LobbyFullScreenWidget.BP_TestChat` (`self.LobbyGUI`)) message))

(event `Key|Enter`
  (params (Key :type "Key Structure"))
  (bind _chattxt (`/DBDUI/Blueprints/BP_TestChat.ChatTxt` (`/DBDUI/Blueprints/Lobby/WBP_LobbyFullScreenWidget.BP_TestChat` (`self.LobbyGUI`))))
  ; 채팅 포커싱
  (:`Pressed`
    (if (not (`Widget.HasKeyboardFocus` _chattxt))
      (`WidgetBlueprintLibrary.SetInputMode_UIOnlyEx` self _chattxt))))

(event `OnAsyncLoadEnd`
  ; 비동기 이벤트 테스트 문장
  (`KismetSystemLibrary.PrintString` "비동기 맵 로딩 완료"))

(event `OnAsyncLoadStart`
  ; 비동기 이벤트 테스트 문장
)

(event `OnSurvivorMatchACK`
  ; 서버 응답 이벤트
  (`/DBDUI/Blueprints/BP_TestChat.SendSystemChat` (`/DBDUI/Blueprints/Lobby/WBP_LobbyFullScreenWidget.BP_TestChat` (`self.LobbyGUI`)) "생존자로 매칭을 시작합니다."))

(event `OnMatchReady`
  (params (matchInfo :type "MatchInfo Structure (by ref)"))
  ; 준비되었으니 맵 로딩 시작
  (`Widget.SetIsEnabled` (`/DBDUI/Blueprints/Lobby/WBP_LobbyFullScreenWidget.WBP_StartButton2` (`self.LobbyGUI`)) false)
  (bind _asd1game_instance (cast `D1GameInstance` (`GameplayStatics.GetGameInstance`)))
  (`D1GameInstance.ClearServerInfo` _asd1game_instance)
  (`D1GameInstance.SetServerInfo` _asd1game_instance matchInfo)
  (bind _asd1net_game_mode (cast `D1NetGameMode` (`GameplayStatics.GetGameMode`)))
  (`D1NetGameMode.LoadAsyncGameMap` _asd1net_game_mode "L_Showcase"))

(event `OnKillerMatchACK`
  ; 서버 응답 이벤트
  (`/DBDUI/Blueprints/BP_TestChat.SendSystemChat` (`/DBDUI/Blueprints/Lobby/WBP_LobbyFullScreenWidget.BP_TestChat` (`self.LobbyGUI`)) "킬러로 매칭을 시작합니다."))

(event `OnMatchCancelACK`
  ; 서버 응답 이벤트
  (`/DBDUI/Blueprints/BP_TestChat.SendSystemChat` (`/DBDUI/Blueprints/Lobby/WBP_LobbyFullScreenWidget.BP_TestChat` (`self.LobbyGUI`)) "매칭이 정상적으로 취소되었습니다."))

(event `OnMatchAbandoned`
  (`/DBDUI/Blueprints/BP_TestChat.SendSystemChat` (`/DBDUI/Blueprints/Lobby/WBP_LobbyFullScreenWidget.BP_TestChat` (`self.LobbyGUI`)) "누군가 나가서 매칭이 취소되었습니다.")
  (`Widget.SetIsEnabled` (`/DBDUI/Blueprints/Lobby/WBP_LobbyFullScreenWidget.WBP_StartButton2` (`self.LobbyGUI`)) true))

(fn `UserConstructionScript`)