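; Repairable generator interactable that exposes its repair progress and switches on its lights with start-up sounds at 100 percent.
; On Tick, the server triggers the light check and starts a looping timer for each newly repairing player, which multicasts electric sparks at that player's hand.
; A separate event spawns an explosion for failed skill checks.
; The completion logic for outline removal and the timed widget is left disconnected.
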(event `self.ReceiveBeginPlay`
  (set `Widget.Visibility` "Hidden" (`WidgetComponent.GetWidget` (`self.WBP_Complete`))))

(event `self.BP_CompleteRepair`)

(event `MultiComplete`
  (params (NewParam :type "/Game/Blueprints/Maps/Interactables/BP_D1Generator Object Reference"))
  (`PrimitiveComponent.SetRenderCustomDepth` (`self.GeneratorMesh`) false)
  (`PrimitiveComponent.SetRenderCustomDepth` (`self.GeneratorLamp`) false))

(event `TurnOnLight_Sound`
  (if (>= (`self.RepairProgress`) 100.0)
    (for _array_element (`|MakeArray` (`self.PointLight`) (`self.PointLight1`) (`self.PointLight2`) (`self.PointLight3`) (`self.SpotLight4`) :!type "PointLightComponent Object Reference")
      (`LightComponent.SetIntensity` _array_element 5000.0)
      (`/Engine/EditorBlueprintResources/StandardMacros.DoOnce` false
        (:`Completed`
          (`GameplayStatics.PlaySoundAtLocation` null (`self.K2_GetActorLocation`) (struct) 1.0 1.0 0.0 "/Game/Art/Sound/Generator/Generator_Piston.Generator_Piston" null null null)
          (`/Engine/EditorBlueprintResources/StandardMacros.DoOnce` false
            (:`Completed`
              (`GameplayStatics.PlaySoundAtLocation` "/Game/Art/Sound/Generator/Generator_Start_Later_Cue.Generator_Start_Later_Cue" (`self.K2_GetActorLocation`) (struct) 1.0 1.0 0.0 "/Game/Art/Sound/Generator/Generator_Piston.Generator_Piston" null null null))))))))

(event `self.ReceiveTick`
  (params (DeltaSeconds :type "Float (single-precision)"))
  (`/Engine/EditorBlueprintResources/ActorMacros.Switch Has Authority`
    (:`Authority`
      (`|ExecutionSequence`
        (:`then_0`
          (`self.TurnOnLight_Sound`))
        (:`then_1`
          (for _array_element (`self.RepairingPlayers`)
            (if (not (`D1SurvivorBase.bPrevRepairing` _array_element))
              (bind _returnvalue (`KismetSystemLibrary.K2_SetTimerDelegate` (delegate `CreateEffect`) 5.0 true))
              (set `self.EffectTime` _returnvalue)
              (set `D1SurvivorBase.bPrevRepairing` true _array_element))))))))

(event `CreateEffect`
  (if (`KismetSystemLibrary.IsValid` (stale `self.ReceiveTick` _array_element))
    (`self.MulticastSpawnEffect` (stale `self.ReceiveTick` _array_element))))

(event `MulticastSpawnEffect`
  (params (Player :type "D1SurvivorBase Object Reference"))
  (bind _mesh (`Character.Mesh` Player))
  (bind _returnvalue_location (`KismetMathLibrary.BreakTransform` (`SceneComponent.GetSocketTransform` _mesh "PlayerHandEffectSocket" "RTS_World")))
  (if (and (`KismetSystemLibrary.IsValid` Player) (`KismetSystemLibrary.IsValid` _mesh))
    (`NiagaraFunctionLibrary.SpawnSystemAtLocation` "/Game/Art/Effect/NS_Electronic.NS_Electronic" (+ (+ _returnvalue_location (0.0 0.0 20.0)) (* (`SceneComponent.GetRightVector` _mesh) 50.0)) (`KismetMathLibrary.ComposeRotators` (`KismetMathLibrary.MakeRotFromX` (`SceneComponent.GetForwardVector` _mesh)) (`KismetMathLibrary.MakeRotator` 0.0 0.0 -90.0)))
    (elif (`KismetSystemLibrary.K2_IsValidTimerHandle` (`self.EffectTime`))
      (`KismetSystemLibrary.K2_ClearAndInvalidateTimerHandle` (`self.EffectTime`)))))

(event `SkillFailEffect`
  (bind _returnvalue_location (`KismetMathLibrary.BreakTransform` (`self.GetTransform`)))
  (`NiagaraFunctionLibrary.SpawnSystemAtLocation` "/Game/Art/Effect/MegaMagicVFXBundle/VFX/MagicalExplosionsVFX/VFX/MagmaExplosion/Systems/N_MagmaExplosion.N_MagmaExplosion" (+ _returnvalue_location (0.0 0.0 20.0))))

(fn `CheckKey`
  (returns (KeyCheck :type Boolean))
  (return false))

(fn `CompleteWidget`
  (if (> (`self.Timer`) 2.0)
    (set `Widget.Visibility` "Hidden" (`WidgetComponent.GetWidget` (`self.WBP_Complete`)))
    (set `self.Timer` 0.0)
    (`KismetSystemLibrary.K2_ClearAndInvalidateTimerHandle` (`self.WidgetTimer`))
    (else
      (set `self.Timer` (+ (`self.Timer`) 0.1)))))

(fn `GetCollisionType`
  (returns (Type :type "/DBDUI/Enum/ECollisionTarget Enum"))
  (return "NewEnumerator3"))

(fn `GetPercent`
  (returns (Percent :type "Float (double-precision)"))
  (return (`self.RepairProgress`)))

(fn `IsInteract`
  (returns (Interact :type Boolean))
  (return false))

(fn `StartEffect`
  (`/Engine/EditorBlueprintResources/ActorMacros.Switch Has Authority`
    (:`Authority`
      (for _array_element (`self.RepairingPlayers`)
        (bind _mesh (`Character.Mesh` _array_element))
        (bind _returnvalue_location (`KismetMathLibrary.BreakTransform` (`SceneComponent.GetSocketTransform` _mesh "PlayerHandEffectSocket" "RTS_World")))
        (`NiagaraFunctionLibrary.SpawnSystemAtLocation` "/Game/Art/Effect/NS_Electronic.NS_Electronic" (+ (+ _returnvalue_location (0.0 0.0 20.0)) (* (`SceneComponent.GetRightVector` _mesh) 50.0)) (`KismetMathLibrary.ComposeRotators` (`KismetMathLibrary.MakeRotFromX` (`SceneComponent.GetForwardVector` _mesh)) (`KismetMathLibrary.MakeRotator` 0.0 0.0 -90.0)))))))

(fn `UpdateInteraction`
  (returns (Percent :type "Float (double-precision)"))
  (return (`self.RepairProgress`)))

(fn `UserConstructionScript`)