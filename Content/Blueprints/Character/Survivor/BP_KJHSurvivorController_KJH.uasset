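; Survivor player controller that adds the in-game full-screen HUD for the local player and runs skill checks during generator repair.
; The repair-start delegate starts a looping timer, its interval randomized once per start, that triggers the HUD skill check and binds its result event.
; CheckSkillFunc reports success or failure to the survivor's current generator, spawning a magma explosion effect just above it on failure.
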(event `self.ReceiveBeginPlay`
  (if (`self.IsLocalController`)
    (bind _returnvalue (`|CreateWidget` "/DBDUI/Blueprints/InGame/WBP_InGameFullScreen.WBP_InGameFullScreen_C"))
    (bind _output_get (set `self.mHUD` _returnvalue))
    (`UserWidget.AddToViewport` _output_get 0)
    (add `self.RepaireStartDelegate` (delegate `RepaireStartDelegate_이벤트`))))

(event `RepaireStartDelegate_이벤트`
  (`self.StartTimer`))

(fn `CheckSkillFunc`
  (params (isSuccess :type Boolean))
  (bind _asd1survivor_base (cast `D1SurvivorBase` (`GameplayStatics.GetPlayerCharacter` 0)))
  (if isSuccess
    (bind _currentgenerator (`D1SurvivorBase.CurrentGenerator` _asd1survivor_base))
    (`D1Generator.OnSkillCheckSuccess` _currentgenerator)
    (`KismetSystemLibrary.PrintString` "Hello")
    (else
      (`D1Generator.OnSkillCheckFail` _currentgenerator null)
      (bind _returnvalue_location (`KismetMathLibrary.BreakTransform` (`self.GetTransform` _currentgenerator)))
      (`NiagaraFunctionLibrary.SpawnSystemAtLocation` "/Game/Art/Effect/MegaMagicVFXBundle/VFX/MagicalExplosionsVFX/VFX/MagmaExplosion/Systems/N_MagmaExplosion.N_MagmaExplosion" (+ _returnvalue_location (0.0 0.0 30.0))))))

(fn `StartSkillCheck`
  (bind _mhud (`self.mHUD`))
  (`/DBDUI/Blueprints/InGame/WBP_InGameFullScreen.StartSkillCheck` _mhud)
  (add `/DBDUI/Blueprints/InGame/WBP_SkillCheck.CheckSuccessEvent` (`/DBDUI/Blueprints/InGame/WBP_InGameFullScreen.SkillCheck` _mhud) (`|CreateDelegate` :!event `CheckSkillFunc`)))

(fn `StartTimer`
  (bind _returnvalue (`KismetSystemLibrary.K2_SetTimer` null "StartSkillCheck" (`KismetMathLibrary.RandomFloatInRange` 3.0 6.0) true))
  (set `self.SkillTimer` _returnvalue))

(fn `UserConstructionScript`)