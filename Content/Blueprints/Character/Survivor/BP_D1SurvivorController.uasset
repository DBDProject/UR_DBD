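; Survivor player controller that drives the in-game HUD, generator repair skill checks and hook skill checks.
; On local BeginPlay it binds game-state, repair and hook delegates, and UnlockInput creates the HUD widget.
; Repairing runs a looping timer, its interval randomized once per start, that triggers skill checks reported to the current generator, with failures forwarded to the server.
; Survivor state changes update the HUD and reset local character effects.
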(event `self.ReceiveBeginPlay`
  (if (`self.IsLocalController`)
    (bind _asbp_d1game_state (cast `/Game/Blueprints/Game/BP_D1GameState` (`GameplayStatics.GetGameState`)))
    (add `D1GameState.OnSurvivorStateChanged` _asbp_d1game_state (`|CreateDelegate` :!event `PlayerChange`))
    (add `D1GameState.OnInputUnlock` _asbp_d1game_state (`|CreateDelegate` :!event `UnlockInput`))
    (add `self.RepaireStartDelegate` (delegate `RepaireStartDelegate_이벤트`))
    (add `self.RepaireEndDelegate` (delegate `RepaireEndDelegate_이벤트`))
    (bind _asbp_d1survivor_base (cast `/Game/Blueprints/Character/Survivor/BP_D1SurvivorBase` (`GameplayStatics.GetPlayerCharacter` 0)))
    (add `/Game/Blueprints/Character/Survivor/BP_D1SurvivorBase.EventGetHookState` _asbp_d1survivor_base (`|CreateDelegate` :!event `PlayerHookCheck`))))

(event `RepaireStartDelegate_이벤트`
  (`self.StartTimer`))

(event `RepaireEndDelegate_이벤트`
  (`self.EndTimer`))

(event `PlayerChange`
  (params (SurvivorIndex :type Integer) (SurvivorState :type "ESurvivorState Enum" :default "None"))
  (`self.OnPlayerChangeState` SurvivorState SurvivorIndex))

(event `OnServerUI`
  (params (TargetActor :type "Actor Object Reference") (IsInteract :type Boolean))
  (bind _asbp_d1survivor_base (cast `/Game/Blueprints/Character/Survivor/BP_D1SurvivorBase` TargetActor))
  (bind _asbp_d1survivor_controller (cast `/Game/Blueprints/Character/Survivor/BP_D1SurvivorController` (`Pawn.GetController` _asbp_d1survivor_base)))
  (`self.OnClientUI` _asbp_d1survivor_controller IsInteract))

(event `OnClientUI`
  (params (NewParam :type Boolean))
  (`/DBDUI/Blueprints/InGame/WBP_InGameFullScreen.InteractOtherPlayer` (`self.mHUD`) NewParam))

(event `UnlockInput`
  (bind _returnvalue (`|CreateWidget` "/DBDUI/Blueprints/InGame/WBP_InGameFullScreen.WBP_InGameFullScreen_C" (`GameplayStatics.GetPlayerController` 0)))
  (bind _output_get (set `self.mHUD` _returnvalue))
  (`UserWidget.AddToViewport` _output_get 0))

(event `Server_Do`
  (params (Generator :type "D1Generator Object Reference"))
  (bind _asbp_d1generator (cast `/Game/Blueprints/Maps/Interactables/BP_D1Generator` Generator))
  (`/Game/Blueprints/Maps/Interactables/BP_D1Generator.SkillFailEffect` _asbp_d1generator))

(event `MultiCastFailEffect`
  (params (Generator :type "D1Generator Object Reference"))
  (bind _returnvalue_location (`KismetMathLibrary.BreakTransform` (`self.GetTransform` Generator)))
  (`NiagaraFunctionLibrary.SpawnSystemAtLocation` "/Game/Art/Effect/MegaMagicVFXBundle/VFX/MagicalExplosionsVFX/VFX/MagmaExplosion/Systems/N_MagmaExplosion.N_MagmaExplosion" (+ _returnvalue_location (0.0 0.0 30.0))))

(fn `CheckSkillFunc`
  (params (isSuccess :type Boolean))
  (bind _asd1survivor_base (cast `D1SurvivorBase` (`GameplayStatics.GetPlayerCharacter` 0)))
  (bind _currentgenerator (`D1SurvivorBase.CurrentGenerator` _asd1survivor_base))
  (if (and (`KismetSystemLibrary.IsValid` _asd1survivor_base) (`KismetSystemLibrary.IsValid` _currentgenerator))
    (if isSuccess
      (`GameplayStatics.PlaySound2D` "/Game/Art/Sound/SkillCheck/AudioEvent_HUD_SkillCheck_Bonus.AudioEvent_HUD_SkillCheck_Bonus" 1.0 1.0 0.0 null null)
      (`D1Generator.OnSkillCheckSuccess` _currentgenerator null)
      (else
        (`D1Generator.OnSkillCheckFail` _currentgenerator _asd1survivor_base)
        (`self.Server_Do` _currentgenerator)))))

(fn `EndTimer`
  (if (`KismetSystemLibrary.K2_IsValidTimerHandle` (`self.Skill Timer`))
    (`KismetSystemLibrary.K2_ClearAndInvalidateTimerHandle` (`self.Skill Timer`))
    (`/DBDUI/Blueprints/InGame/WBP_InGameFullScreen.EndSkillCheck` (`self.mHUD`))))

(fn `OnPlayerChangeState`
  (params (CurrentState :type "ESurvivorState Enum" :default "None") (PlayerIndex :type Integer))
  (`/DBDUI/Blueprints/InGame/WBP_InGameFullScreen.ChangePlayerState` (`self.mHUD`) CurrentState PlayerIndex)
  (bind _asbp_d1survivor_base (cast `/Game/Blueprints/Character/Survivor/BP_D1SurvivorBase` (`GameplayStatics.GetPlayerPawn` 0)))
  (if (== PlayerIndex (`D1SurvivorBase.PlayerIndex` _asbp_d1survivor_base))
    (switch `ESurvivorState` CurrentState
      (:`Healthy`
        (`/Game/Blueprints/Character/Survivor/BP_D1SurvivorBase.ResetAll` _asbp_d1survivor_base))
      (:`Injured`
        (`/Game/Blueprints/Character/Survivor/BP_D1SurvivorBase.ResetAll` _asbp_d1survivor_base)
        (`/Game/Blueprints/Character/Survivor/BP_D1SurvivorBase.ControllerEffect` _asbp_d1survivor_base)
        (`/DBDUI/Blueprints/Player/WBP_InGamePlayerInfoWidget.UnSwitchActive` (`|GetArrayItem` (`/DBDUI/Blueprints/InGame/WBP_InGameFullScreen.WBP_PlayerInfo` (`self.mHUD`)) PlayerIndex)))
      (:`Crawl`
        (`/Game/Blueprints/Character/Survivor/BP_D1SurvivorBase.ResetAll` _asbp_d1survivor_base)
        (`/Game/Blueprints/Character/Survivor/BP_D1SurvivorBase.ControllerEffect` _asbp_d1survivor_base))
      (:`PickedUp`
        (`/Game/Blueprints/Character/Survivor/BP_D1SurvivorBase.ResetAll` _asbp_d1survivor_base))
      (:`Hooked`
        (`/Game/Blueprints/Character/Survivor/BP_D1SurvivorBase.ResetAll` _asbp_d1survivor_base)
        (`/DBDUI/Blueprints/Player/WBP_InGamePlayerInfoWidget.SwitchActive` (`|GetArrayItem` (`/DBDUI/Blueprints/InGame/WBP_InGameFullScreen.WBP_PlayerInfo` (`self.mHUD`)) PlayerIndex))))))

(fn `PlayerHookCheck`
  (params (IsState :type Boolean))
  (bind _mhud (`self.mHUD`))
  (bind _d1survivor (`self.D1Survivor`))
  (if IsState
    (if (and (`KismetSystemLibrary.IsValid` _d1survivor) (`|EnumEquality` (`D1SurvivorBase.CurrentState` _d1survivor) "Hooked"))
      (`GameplayStatics.PlaySound2D` "/Game/Art/Sound/SkillCheck/AudioEvent_HUD_SkillCheck_Overcharge.AudioEvent_HUD_SkillCheck_Overcharge" 1.0 1.0 0.0 null null)
      (`/DBDUI/Blueprints/InGame/WBP_InGameFullScreen.StartHookSkillCheck` _mhud)
      (else
        (`/DBDUI/Blueprints/InGame/WBP_InGameFullScreen.EndHookSkill` _mhud :!label _label)))
    (else
      (goto _label))))

(fn `StartSkillCheck`
  (bind _mhud (`self.mHUD`))
  (bind _d1survivor (`self.D1Survivor`))
  (bind _currentstate (`D1SurvivorBase.CurrentState` _d1survivor))
  (if (and (and (`KismetSystemLibrary.IsValid` _d1survivor) (or (`|EnumEquality` _currentstate "Healthy") (`|EnumEquality` _currentstate "Injured"))) (`D1SurvivorBase.bIsRepairing` _d1survivor))
    (`GameplayStatics.PlaySound2D` "/Game/Art/Sound/SkillCheck/AudioEvent_HUD_SkillCheck_Overcharge.AudioEvent_HUD_SkillCheck_Overcharge" 1.0 1.0 0.0 null null)
    (`/DBDUI/Blueprints/InGame/WBP_InGameFullScreen.StartSkillCheck` _mhud)
    (add `/DBDUI/Blueprints/InGame/WBP_SkillCheck.CheckSuccessEvent` (`/DBDUI/Blueprints/InGame/WBP_InGameFullScreen.SkillCheck` _mhud) (`|CreateDelegate` :!event `CheckSkillFunc`))))

(fn `StartTimer`
  (bind _returnvalue (`KismetSystemLibrary.K2_SetTimer` null "StartSkillCheck" (`KismetMathLibrary.RandomFloatInRange` 3.0 6.0) true))
  (set `self.Skill Timer` _returnvalue))

(fn `UserConstructionScript`)