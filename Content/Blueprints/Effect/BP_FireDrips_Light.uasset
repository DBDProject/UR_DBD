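; BP_FireDrips_Light is a fire effect actor with a point light and an intermittent drip particle emitter.
; On BeginPlay it loops endlessly, waiting a random delay, enabling the FireEffect "Drip" emitter for a random duration, then disabling it.
; The construction script applies configurable color, intensity, radius, shadow casting and a relative position offset to the light, which the drip loop leaves untouched.
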(event `self.ReceiveBeginPlay`
  (`KismetSystemLibrary.Delay` (`KismetMathLibrary.RandomFloatInRange` (`self.Drip Delay Min`) (`self.Drip Delay Max`)) :!label _label)
  (`ParticleSystemComponent.SetEmitterEnable` (`self.FireEffect`) "Drip" true)
  (`KismetSystemLibrary.Delay` (`KismetMathLibrary.RandomFloatInRange` (`self.Drip Time Min`) (`self.Drip Time Max`)))
  (`ParticleSystemComponent.SetEmitterEnable` (`self.FireEffect`) "Drip" false)
  (`self.OnLoop`))

(event `OnLoop`
  (goto _label))

(fn `UserConstructionScript`
  (bind _pointlightfire (`self.PointLightFire`))
  ;[1 1 1] Light Settings
  (`LightComponent.SetLightColor` _pointlightfire (`self.LightFireColor`) true)
  (`LightComponent.SetIntensity` _pointlightfire (`self.LightIntensity`))
  (`PointLightComponent.SetAttenuationRadius` _pointlightfire (`self.LightRadius`))
  (`LightComponentBase.SetCastShadows` _pointlightfire (`self.Cast Shadows`))
  (`SceneComponent.K2_AddRelativeLocation` _pointlightfire (`self.PointLightLoc`) false false))