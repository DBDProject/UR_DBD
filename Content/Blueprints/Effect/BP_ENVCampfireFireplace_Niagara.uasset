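; Campfire or fireplace effect actor that pairs a Niagara fire effect with a point light.
; The construction script applies exposed variables to the light's color, intensity, radius, shadow casting and relative offset.
; It also feeds fire, ember and smoke colors plus intensity and ember lerp offset into Niagara parameters, with the fire color shared by light and particles.
; The event graph holds no active logic.
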(fn `UserConstructionScript`
  (bind _niagarafirefx (`self.NiagaraFireFX`))
  (bind _pointlightfire (`self.PointLightFire`))
  (bind _lightfirecolor (`self.LightFireColor`))
  ;[1 1 1] Light Settings
  (`LightComponent.SetLightColor` _pointlightfire _lightfirecolor true)
  (`LightComponent.SetIntensity` _pointlightfire (`self.LightIntensity`))
  (`PointLightComponent.SetAttenuationRadius` _pointlightfire (`self.LightRadius`))
  (`LightComponentBase.SetCastShadows` _pointlightfire (`self.Cast Shadows`))
  (`SceneComponent.K2_AddRelativeLocation` _pointlightfire (`self.PointLightLoc`) false false)
  ;[1 1 1] Particle Settings
  (`ParticleSystemComponent.SetColorParameter` _niagarafirefx "FireColor" _lightfirecolor)
  (`NiagaraComponent.SetVariableFloat` _niagarafirefx "FireColorIntesnityScale" (`self.FireIntensity`))
  (`FXSystemComponent.SetColorParameter` _niagarafirefx "EndEmberColor" (`self.End Ember Color`))
  (`NiagaraComponent.SetVariableFloat` _niagarafirefx "LerpOffset" (`self.EmberColorOffset`))
  (`ParticleSystemComponent.SetColorParameter` _niagarafirefx "SmokeColor" (`self.SmokeColor`)))