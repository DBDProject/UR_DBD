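; Candle flame effect Blueprint with a configurable point light for the fire's glow.
; The Construction Script copies exposed-style variables for color, intensity, attenuation radius and shadow casting onto PointLightFire.
; It then shifts the light by PointLightLoc as a relative offset added to its current position, rather than setting an absolute location.
; The graph shown holds only this setup, with no runtime flicker logic.
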(fn `UserConstructionScript`
  (bind _pointlightfire (`self.PointLightFire`))
  ;[1 1 1] Light Settings
  (`LightComponent.SetLightColor` _pointlightfire (`self.LightFireColor`) true)
  (`LightComponent.SetIntensity` _pointlightfire (`self.LightIntensity`))
  (`PointLightComponent.SetAttenuationRadius` _pointlightfire (`self.LightRadius`))
  (`LightComponentBase.SetCastShadows` _pointlightfire (`self.Cast Shadows`))
  (`SceneComponent.K2_AddRelativeLocation` _pointlightfire (`self.PointLightLoc`) false false))