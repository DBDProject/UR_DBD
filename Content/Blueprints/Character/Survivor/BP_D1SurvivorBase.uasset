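; Base survivor character Blueprint that leaves footstep and blood decals while the survivor runs.
; Tick watches velocity on the locally controlled player and starts or clears a looping timer as a speed threshold is crossed.
; A Server, ServerEffect and OnFootSetpEffectMulti event chain spawns both decals behind the player with random sideways jitter.
; It also line-traces to a random left or right side, placing another footstep decal on any surface hit.
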(event `self.ReceiveTick`
  (params (DeltaSeconds :type "Float (single-precision)"))
  (bind _prevrunstate (`self.PrevRunState`))
  (bind `_as플레이어_컨트롤러` (cast `PlayerController` (`self.GetController`)))
  (if (`Controller.IsLocalPlayerController` (`GameplayStatics.GetPlayerController` (`GameplayStatics.GetPlayerControllerID` `_as플레이어_컨트롤러`)))
    (if (>= (`KismetMathLibrary.VSize` (`MovementComponent.Velocity` (`self.CharacterMovement`))) 256.0)
      (if (not _prevrunstate)
        (set `self.PrevRunState` true)
        (bind _returnvalue (`KismetSystemLibrary.K2_SetTimerDelegate` (`|CreateDelegate` :!event `Server`) 0.5 true))
        (set `self.FootSetpTimer` _returnvalue)
        (set `self.EventPlayer` null))
      (elif _prevrunstate
        (set `self.PrevRunState` false)
        (`KismetSystemLibrary.K2_ClearAndInvalidateTimerHandle` (`self.FootSetpTimer`))))))

(event `Server`
  (`self.ServerEffect` self))

(event `ServerEffect`
  (params (Player :type "Actor Object Reference"))
  (`self.OnFootSetpEffectMulti` Player))

(event `OnFootSetpEffectMulti`
  (params (Player :type "Actor Object Reference"))
  (bind _returnvalue (`KismetMathLibrary.RandomFloatInRange` -20.0 20.0))
  (`|SpawnActorFromClass` "/DBDUI/Blueprints/Decal/BP_FootSetpBloodDecal.BP_FootSetpBloodDecal_C" (`KismetMathLibrary.Conv_VectorToTransform` (+ (- (`self.K2_GetActorLocation` Player) (`KismetMathLibrary.MakeVector` 0.0 _returnvalue 92.0)) (* (`self.GetActorForwardVector` Player) -120.0))) "Undefined" "MultiplyWithRoot" null null)
  (`|SpawnActorFromClass` "/DBDUI/Blueprints/Decal/BP_FootSetpDecal.BP_FootSetpDecal_C" (`KismetMathLibrary.Conv_VectorToTransform` (+ (- (`self.K2_GetActorLocation` Player) (`KismetMathLibrary.MakeVector` 0.0 _returnvalue 92.0)) (* (`self.GetActorForwardVector` Player) -120.0))) "Undefined" "MultiplyWithRoot" null null)
  (bind (_ishit _location _normalparam) (`self.TraceSpawnNormal` Player))
  (if _ishit
    (`|SpawnActorFromClass` "/DBDUI/Blueprints/Decal/BP_FootSetpDecal.BP_FootSetpDecal_C" (`KismetMathLibrary.MakeTransform` (`KismetMathLibrary.MakeVector` (.x _location) (.y _location) (.z _location)) (`KismetMathLibrary.Conv_VectorToRotator` (+ _normalparam (`KismetMathLibrary.MakeRotator` 0.0 90.0)))) "Undefined" "MultiplyWithRoot" null null)))

(fn `OnFootSetpEffect`)

(fn `TraceSpawnNormal`
  (params (Player :type "Actor Object Reference"))
  (returns (IsHit :type Boolean) (Location :type "Vector Structure") (NormalParam :type "Vector Structure"))
  (locals (y :type "Float (double-precision)" :default 0.0))
  (bind _returnvalue (`KismetMathLibrary.RandomIntegerInRange` 0 1))
  (if (== (`KismetMathLibrary.SelectFloat` (`KismetMathLibrary.Conv_IntToDouble` _returnvalue) (`KismetMathLibrary.Conv_IntToDouble` _returnvalue)) 0.0)
    (set `local.y` 250.0)
    (else
      (set `local.y` -250.0)))
  (bind (_outhit _returnvalue_2) (`KismetSystemLibrary.LineTraceSingle` (`KismetMathLibrary.MakeVector` (.x (`self.K2_GetActorLocation` Player)) (.y (`self.K2_GetActorLocation` Player)) (+ (.z (`self.K2_GetActorLocation` Player)) 20.0)) (`KismetMathLibrary.TransformLocation` (`self.GetTransform`) (`KismetMathLibrary.MakeVector` 0.0 (`local.y`))) "TraceTypeQuery1" true))
  (return _returnvalue_2 (`.Location` (`GameplayStatics.BreakHitResult` _outhit)) (`.Normal` (`GameplayStatics.BreakHitResult` _outhit))))

(fn `UserConstructionScript`)