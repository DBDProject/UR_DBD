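; BP_D1Pallet is an interactable pallet actor with Up, Down and Destroyed states.
; GetCollisionType maps the current state to a collision type enum value.
; Tick draws colored debug spheres at the left, right and center interaction points every frame.
; CheckKey, IsInteract, GetPercent and UpdateInteraction return only false or zero, so the Blueprint itself holds no interaction logic.
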(event `self.ReceiveTick`
  (params (DeltaSeconds :type "Float (single-precision)"))
  (`KismetSystemLibrary.DrawDebugSphere` (`SceneComponent.K2_GetComponentLocation` (`self.InteractionPoint_Left`)) 20.0 12 (struct :`R` 1.0 :`B` 0.097826 :`A` 1.0))
  (`KismetSystemLibrary.DrawDebugSphere` (`SceneComponent.K2_GetComponentLocation` (`self.InteractionPoint_Right`)) 20.0 12 (struct :`R` 0.208059 :`G` 1.0 :`B` 0.278838 :`A` 1.0))
  (`KismetSystemLibrary.DrawDebugSphere` (`SceneComponent.K2_GetComponentLocation` (`self.InteractionPoint_Center`)) 20.0 12 (struct :`R` 1.0 :`G` 0.938499 :`A` 1.0)))

(fn `CheckKey`
  (returns (KeyCheck :type Boolean))
  (return false))

(fn `GetCollisionType`
  (returns (Type :type "/DBDUI/Enum/ECollisionTarget Enum"))
  (switch `EPalletState` (`self.CurrentState`)
    (:`Up`
      (return "NewEnumerator0"))
    (:`Down`
      (return "NewEnumerator5"))
    (:`Destroyed`
      (return "NewEnumerator4"))))

(fn `GetPercent`
  (returns (Percent :type "Float (double-precision)"))
  (return 0.0))

(fn `IsInteract`
  (returns (Interact :type Boolean))
  (return false))

(fn `UpdateInteraction`
  (returns (Percent :type "Float (double-precision)"))
  (return 0.0))

(fn `UserConstructionScript`)