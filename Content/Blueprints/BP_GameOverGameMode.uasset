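; BP_GameOverGameMode is a game mode Blueprint that builds a chain of GroundSpawner tiles.
; On BeginPlay it takes the first GroundSpawner found in the level, gives it a reference to itself and spawns three more from that tile's SpawnPoint.
; SpawnTiles places each new tile at the previous one's SpawnPoint, passes it the game mode reference and saves the next spawn location.
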(event `self.ReceiveBeginPlay`
  (bind _outactors (`GameplayStatics.GetAllActorsOfClass` "/Game/Blueprints/Maps/GameOver/GroundSpawner.GroundSpawner_C"))
  (bind _output_get (set `self.BaseTile_Ref` (`|GetArrayItem` _outactors)))
  (set `/Game/Blueprints/Maps/GameOver/GroundSpawner.GameMode_ref` self _output_get)
  (set `self.Next_Spawn_Point` (`SceneComponent.K2_GetComponentLocation` (`/Game/Blueprints/Maps/GameOver/GroundSpawner.SpawnPoint` _output_get)))
  (`self.Spawn_Tiles` 3))

(fn `Spawn_Tiles`
  (params (Amount :type Integer))
  (for _ (range Amount)
    (bind _returnvalue (`|SpawnActorFromClass` "/Game/Blueprints/Maps/GameOver/GroundSpawner.GroundSpawner_C" (`KismetMathLibrary.MakeTransform` (`self.Next_Spawn_Point`)) "Undefined" "MultiplyWithRoot" null null))
    (set `/Game/Blueprints/Maps/GameOver/GroundSpawner.GameMode_ref` self _returnvalue)
    (set `self.Next_Spawn_Point` (`SceneComponent.K2_GetComponentLocation` (`/Game/Blueprints/Maps/GameOver/GroundSpawner.SpawnPoint` _returnvalue)))))

(fn `UserConstructionScript`)