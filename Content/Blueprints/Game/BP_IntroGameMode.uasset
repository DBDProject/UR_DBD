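; Intro game mode that opens the network connection at startup and then moves the player to the lobby.
; On BeginPlay it gets the net manager from D1GameInstance and connects to a hardcoded localhost server.
; It prints success, or failure with a debug-mode notice, then loads LobbyMap after a short delay in either case.
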(event `self.ReceiveBeginPlay`
  (bind _asd1game_instance (cast `D1GameInstance` (`GameplayStatics.GetGameInstance`)))
  (bind _returnvalue (`D1GameInstance.GetNetManager` _asd1game_instance))
  (bind _returnvalue_2 (`DBDNetManager.Connect` _returnvalue "127.0.0.1" 5000))
  (if _returnvalue_2
    (`KismetSystemLibrary.PrintString` "서버 접속 성공" true true (struct :`G` 0.66 :`B` 1.0 :`A` 1.0) 5.0)
    (`KismetSystemLibrary.Delay` 3.0)
    (`GameplayStatics.OpenLevel` "LobbyMap")
    (else
      (`KismetSystemLibrary.PrintString` "서버 접속 실패 디버그 모드로 진입" true true (struct :`G` 0.66 :`B` 1.0 :`A` 1.0) 5.0)
      (`KismetSystemLibrary.Delay` 3.0)
      (`GameplayStatics.OpenLevel` "LobbyMap"))))

(fn `UserConstructionScript`)