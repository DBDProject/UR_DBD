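; Player controller for the Dracula killer character that manages the killer's full-screen in-game HUD.
; On BeginPlay, the local controller binds to the D1GameState events for input unlock and survivor state changes.
; Input unlock creates WBP_InGameFullScreen_Killer and adds it to the viewport.
; Survivor state changes are forwarded to that HUD by player index, with no check that the widget exists yet.
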(event `self.ReceiveBeginPlay`
  (if (`self.IsLocalController`)
    (bind _asd1game_state (cast `D1GameState` (`GameplayStatics.GetGameState`)))
    (add `D1GameState.OnInputUnlock` _asd1game_state (`|CreateDelegate` :!event `UnlockInput`))
    (add `D1GameState.OnSurvivorStateChanged` _asd1game_state (`|CreateDelegate` :!event `PlayerStateChange`))))

(event `PlayerStateChange`
  (params (SurvivorIndex :type Integer) (SurvivorState :type "ESurvivorState Enum" :default "None"))
  (`/DBDUI/Blueprints/InGame/WBP_InGameFullScreen_Killer.OnChangePlayerState` (`self.HUD`) SurvivorState SurvivorIndex))

(event `UnlockInput`
  (bind _returnvalue (`|CreateWidget` "/DBDUI/Blueprints/InGame/WBP_InGameFullScreen_Killer.WBP_InGameFullScreen_Killer_C" self))
  (bind _output_get (set `self.HUD` _returnvalue))
  (`UserWidget.AddToViewport` _output_get 0))

(fn `UserConstructionScript`)