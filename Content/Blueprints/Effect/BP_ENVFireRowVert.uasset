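; BP_ENVFireRowVert is an environment fire effect that pairs a particle system with a point light.
; Its construction script applies exposed variables to the light's color, intensity, radius, shadows and relative offset.
; It also pushes color, intensity and alpha values for fire and smoke into named particle parameters.
; One color variable drives both the light and the flames, keeping them matched.
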(fn `UserConstructionScript`
  (bind _fireeffect (`self.FireEffect`))
  (bind _pointlightfire (`self.PointLightFire`))
  (bind _lightfirecolor (`self.LightFireColor`))
  ;[1 1 1] Light Settings
  (`LightComponent.SetLightColor` _pointlightfire _lightfirecolor true)
  (`LightComponent.SetIntensity` _pointlightfire (`self.LightIntensity`))
  (`PointLightComponent.SetAttenuationRadius` _pointlightfire (`self.LightRadius`))
  (`LightComponentBase.SetCastShadows` _pointlightfire (`self.Cast Shadows`))
  (`SceneComponent.K2_AddRelativeLocation` _pointlightfire (`self.PointLightLoc`) false false)
  ;[1 1 1] Particle Settings
  (`ParticleSystemComponent.SetColorParameter` _fireeffect "FireColor" _lightfirecolor)
  (`ParticleSystemComponent.SetFloatParameter` _fireeffect "FireColorIntesnityScale" (`self.FireIntensity`))
  (`ParticleSystemComponent.SetFloatParameter` _fireeffect "FireAlphaMultScale" (`self.FireAlphaIntensity`))
  (`ParticleSystemComponent.SetColorParameter` _fireeffect "SmokeColor" (`self.SmokeColor`))
  (`ParticleSystemComponent.SetFloatParameter` _fireeffect "SmokeColorScale" (`self.SmokeColorIntensity`))
  (`ParticleSystemComponent.SetFloatParameter` _fireeffect "SmokeAlphaScale" (`self.SmokeAlphaScale`)))