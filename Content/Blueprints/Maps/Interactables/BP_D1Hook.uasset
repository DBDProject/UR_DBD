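; BP_D1Hook is a map interactable representing a hook, with collision that depends on whether it is hooked.
; GetCollisionType returns one of two enum values based on the IsHooked flag.
; CheckKey, IsInteract, GetPercent and UpdateInteraction are stubs returning false or zero, so it offers no interaction or progress of its own.
; The event graph and construction script are empty, and nothing in this Blueprint sets IsHooked.
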(fn `CheckKey`
  (returns (KeyCheck :type Boolean))
  (return false))

(fn `GetCollisionType`
  (returns (Type :type "/DBDUI/Enum/ECollisionTarget Enum"))
  (if (`self.bIsHooked`)
    (return "NewEnumerator1")
    (else
      (return "NewEnumerator10"))))

(fn `GetPercent`
  (returns (Percent :type "Float (double-precision)"))
  (return 0.0))

(fn `IsInteract`
  (returns (Interact :type Boolean))
  (return false))

(fn `UpdateInteraction`
  (returns (Percent :type "Float (double-precision)"))
  (return 0.0))

(fn `UserConstructionScript`)